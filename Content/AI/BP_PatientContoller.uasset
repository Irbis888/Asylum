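; BP_PatientContoller is an AI controller, apparently for patient characters, that keeps a task-in-progress flag up to date on its Blackboard.
; Every Tick it compares the Time and TaskEnd integer keys and writes DoingTask as true while Time is less than TaskEnd.
; BeginPlay is disabled, and the graph neither starts a behavior tree nor sets those two time keys.
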(event `self.ReceiveTick`
  (params (DeltaSeconds :type "Float (single-precision)"))
  (bind _returnvalue (`AIBlueprintHelperLibrary.GetBlackboard` null))
  (`parent.ReceiveTick` DeltaSeconds)
  (`BlackboardComponent.SetValueAsBool` _returnvalue "DoingTask" (< (`BlackboardComponent.GetValueAsInt` _returnvalue "Time") (`BlackboardComponent.GetValueAsInt` _returnvalue "TaskEnd"))))

(fn `UserConstructionScript`
  (`parent.UserConstructionScript`))
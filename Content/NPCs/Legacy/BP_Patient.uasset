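; Patient NPC that follows a daily timetable of timed tasks, registering with the observer controller and adding its own schedule editor widget to the time UI.
; A looping timer, scaled by the UI speed setting, checks game time against the timetable, choosing the latest-starting matching task or the next start time.
; The resulting busy state and task type are written to the AI blackboard and shown on the task label.
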(event `self.ReceiveBeginPlay`
  (bind _schcontainer (`/Game/UI/WB_HUD.SchContainer` (`/Game/Characters/BP_ObsController.TimeWidget` (`self.PContr`))))
  (`parent.ReceiveBeginPlay`)
  (bind _output_get (set `self.PContr` (cast `/Game/Characters/BP_ObsController` (`GameplayStatics.GetPlayerController` 0) :!pure true)))
  (`KismetSystemLibrary.DelayUntilNextTick`)
  (`KismetSystemLibrary.K2_SetTimerDelegate` (delegate `TimeChanged`) (/ 1.0 (* (`KismetMathLibrary.Conv_IntToDouble` (`/Game/UI/WB_HUD.SpeedScale` (`/Game/Characters/BP_ObsController.TimeWidget` _output_get))) 0.5)) true)
  (bind _keys (`BlueprintMapLibrary.Map_Keys` (`self.TimeTable`)))
  (set `self.TimeToCheck` (`.MinValue` (`KismetMathLibrary.MinOfIntArray` _keys)))
  (`KismetArrayLibrary.Array_Add` (`/Game/Characters/BP_ObsController.PatientList` (`self.PContr`)) self)
  (bind _returnvalue (`|CreateWidget` "/Game/UI/WB_ScheduleEditor.WB_ScheduleEditor_C" (`self.PContr`) (`self.TimeTable`) self))
  (bind _output_get_2 (set `self.ScheduleWidget` _returnvalue))
  (`/Game/UI/WB_ScheduleEditor.MakeTable` _output_get_2)
  (`PanelWidget.AddChild` _schcontainer (`self.ScheduleWidget`))
  (`Widget.SetVisibility` _schcontainer "Visible"))

(event `self.ReceiveTick`
  (params (DeltaSeconds :type "Float (single-precision)"))
  (`parent.ReceiveTick` DeltaSeconds))

(event `TimeChanged`
  (bind _time (`/Game/Characters/BP_ObsController.Time` (`self.PContr`)))
  (if (and (>= _time (`self.TimeToCheck`)) true)
    (bind (_task _schedule) (`self.CheckTime` _time))
    (if _schedule
      (set `self.TimeToCheck` (+ _time (break `/Game/TimetableStuff/Tech/STR_Todo` _task)))
      (set `self.Task Type` (`.Task_9_7041C5964D728D93B1BC5C909A164F65` (break `/Game/TimetableStuff/Tech/STR_Todo` _task)))
      (set `self.Busy` true)
      (else
        (set `self.Busy` false)
        (bind _nexttime (`self.NextTask` _time))
        (set `self.TimeToCheck` (+ (* (/ (`/Game/Characters/BP_ObsController.Time` (`self.PContr`)) 1440) 1440) _nexttime))))
    (`self.FillBB`)))

(event `FillBB`
  (bind _busy (`self.Busy`))
  (bind _task_type (`self.Task Type`))
  (bind _tasklabel (`self.TaskLabel`))
  (bind _returnvalue (`AIBlueprintHelperLibrary.GetBlackboard` (`AIBlueprintHelperLibrary.GetAIController` self)))
  (`|ExecutionSequence`
    (:`then_0`
      (`BlackboardComponent.SetValueAsBool` _returnvalue "DoingTask" _busy))
    (:`then_1`
      (`BlackboardComponent.SetValueAsEnum` _returnvalue "TaskType" _task_type)
      (if _busy
        (`TextRenderComponent.K2_SetText` _tasklabel (`KismetTextLibrary.Conv_StringToText` (`|GetEnumeratorNameAsString` _task_type)))
        (else
          (`TextRenderComponent.K2_SetText` _tasklabel (`KismetTextLibrary.Conv_BoolToText` _busy)))))))

(fn `CheckTime`
  (params (Time :type Integer))
  (returns (Task :type "/Game/TimetableStuff/Tech/STR_Todo Structure") (Schedule :type Boolean))
  (locals (MapKeys :type "Array of Integer") (StartTime :type Integer :default -1))
  (bind _starttime (`local.StartTime`))
  (bind _value (`BlueprintMapLibrary.Map_Find` (`self.TimeTable`) _starttime))
  (bind _returnvalue (== _starttime -1))
  (bind _returnvalue_2 (not _returnvalue))
  (bind _keys (`BlueprintMapLibrary.Map_Keys` (`self.TimeTable`)))
  (bind _output_get (set `local.MapKeys` _keys))
  (for _array_element _output_get
    (if (`self.CheckOption` (mod Time 1440) _array_element (break `/Game/TimetableStuff/Tech/STR_Todo` (`BlueprintMapLibrary.Map_Find` (`self.TimeTable`) _array_element)))
      (set `local.StartTime` (`KismetMathLibrary.Max` (`local.StartTime`) _array_element))))
  (if _returnvalue
    (return (make `/Game/TimetableStuff/Tech/STR_Todo` 10 "NewEnumerator3") _returnvalue_2)
    (else
      (`KismetSystemLibrary.PrintString` (`|GetEnumeratorNameAsString` (`.Task_9_7041C5964D728D93B1BC5C909A164F65` (break `/Game/TimetableStuff/Tech/STR_Todo` _value))))
      (return _value _returnvalue_2))))

(fn `NextTask`
  (params (C :type Integer))
  (returns (NextTime :type Integer))
  (locals (Out :type Integer :default 1440))
  (bind _returnvalue (mod C 1440))
  (bind _keys (`BlueprintMapLibrary.Map_Keys` (`self.TimeTable`)))
  (if (> _returnvalue (`.MaxValue` (`KismetMathLibrary.MaxOfIntArray` _keys)))
    (return (`.MinValue` (`KismetMathLibrary.MinOfIntArray` _keys)))
    (else
      (for _array_element _keys
        (if (>= _array_element _returnvalue)
          (set `local.Out` (`KismetMathLibrary.Min` _array_element (`local.Out`)))))
      (return (`local.Out`)))))

(fn `UserConstructionScript`
  (`parent.UserConstructionScript`))